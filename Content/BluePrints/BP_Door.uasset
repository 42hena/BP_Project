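; BP_Door is a door actor that the player character can break by ramming it at speed.
; On Hit, unless flagged Fake, it checks the horizontal velocity of a colliding BP_ThirdPersonCharacter against a speed threshold.
; Each fast enough impact lowers HealthPower and prints the speed, and the door destroys itself once health drops below zero.
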(event EventBeginPlay)

(event Collision|EventActorBeginOverlap
  (params (OtherActor :type Actor%20Object%20Reference)))

(event EventTick
  (params (DeltaSeconds :type Float%20%28single-precision%29)))

(event Collision|EventHit
  (params (MyComp :type Primitive%20Component%20Object%20Reference) (Other :type Actor%20Object%20Reference) (OtherComp :type Primitive%20Component%20Object%20Reference) (bSelfMoved :type Boolean) (HitLocation :type Vector :default "0, 0, 0") (HitNormal :type Vector :default "0, 0, 0") (NormalImpulse :type Vector :default "0, 0, 0") (Hit :type Hit%20Result%20Structure%20%28by%20ref%29))
  (if (not (Variables|Default|GetbFake))
    (bind _asbp_third_person_character (Utilities|Casting|CastToBP_ThirdPersonCharacter Other))
    (if (>= (Math|Vector|VectorLengthXY (Variables|/Script/Engine.MovementComponent|GetVelocity (Variables|/Script/Engine.Character|GetCharacterMovement _asbp_third_person_character))) 5e+02)
      (bind _output_get (Variables|Default|SetHealthPower (- (Variables|Default|GetHealthPower) 1e+01)))
      (Development|PrintString (Utilities|String|ToString(Float) (Math|Vector|VectorLengthXY (Variables|/Script/Engine.MovementComponent|GetVelocity (Variables|/Script/Engine.Character|GetCharacterMovement _asbp_third_person_character)))))
      (if (< _output_get 0.0)
        (Actor|DestroyActor)))))

(fn ConstructionScript)
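; BP_Cannon is a cannon actor that automatically fires BP_CannonProjectile cannonballs at a repeating interval.
; Tick accumulates delta time and, once it exceeds Timer, resets it and fires unless the Test flag is set.
; Each shot prints a debug message, spawns the projectile ahead along the Arrow's forward vector from the location cached at BeginPlay, and launches its Sphere with a velocity-change impulse.
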(event EventBeginPlay
  (Variables|Default|SetLocation (Transformation|GetActorLocation)))

(event Collision|EventActorBeginOverlap
  (params (OtherActor :type Actor%20Object%20Reference)))

(event EventTick
  (params (DeltaSeconds :type Float%20%28single-precision%29))
  (bind _arrow (Variables|Default|GetArrow))
  (bind _returnvalue (Math|Vector|GetForwardVector _arrow))
  (Variables|Default|SetdeltaTime (+ (Variables|Default|GetdeltaTime) DeltaSeconds))
  (if (< (Variables|Default|GetTimer) (Variables|Default|GetdeltaTime))
    (Variables|Default|SetdeltaTime 0.0)
    (if (not (Variables|Default|Gettest))
      (Development|PrintString "대포알 생성")
      (bind _returnvalue_2 (Game|SpawnActorfromClass "/Game/BluePrints/Cannon/BP_CannonProjectile.BP_CannonProjectile_C" (Math|Conversions|ToTransform(Vector) (+ (* _returnvalue 3e+02) (Variables|Default|GetLocation))) "Undefined" "MultiplyWithRoot" 0 0))
      (Physics|AddImpulse (Variables|/Game/BluePrints/Cannon/BP_CannonProjectile.BP_CannonProjectile_C|GetSphere _returnvalue_2) (+ "" (* _returnvalue 1e+03)) "None" true))))

(fn ConstructionScript)
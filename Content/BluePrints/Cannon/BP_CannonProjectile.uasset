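; BP_CannonProjectile is a cannon projectile that knocks back the third-person character it hits.
; The Hit event casts the other actor to BP_ThirdPersonCharacter and launches it along the inverted, horizontally flattened hit normal, adding to its current velocity.
; Tick is empty, and leftover lifetime-destroy, forward-impulse and debug-print logic is disconnected, so this graph neither moves nor destroys the projectile.
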(event EventBeginPlay)

(event Collision|EventActorBeginOverlap
  (params (OtherActor :type Actor%20Object%20Reference)))

(event EventTick
  (params (DeltaSeconds :type Float%20%28single-precision%29)))

(event Collision|EventHit
  (params (MyComp :type Primitive%20Component%20Object%20Reference) (Other :type Actor%20Object%20Reference) (OtherComp :type Primitive%20Component%20Object%20Reference) (bSelfMoved :type Boolean) (HitLocation :type Vector :default "0, 0, 0") (HitNormal :type Vector :default "0, 0, 0") (NormalImpulse :type Vector :default "0, 0, 0") (Hit :type Hit%20Result%20Structure%20%28by%20ref%29))
  (bind (_x _y) (Math|Vector|BreakVector HitNormal))
  (bind _asbp_third_person_character (Utilities|Casting|CastToBP_ThirdPersonCharacter Other))
  (Character|LaunchCharacter _asbp_third_person_character (* (Math|Vector|MakeVector _x _y 0.0) -1e+03) false false))

(fn ConstructionScript)
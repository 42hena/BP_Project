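; Obstacle ball that knocks BP_ThirdPersonCharacter away on contact.
; Any actor overlap applies a Z-axis torque to the KnokbackBall component.
; On a component hit with the character, it prints the impact normal and calls LaunchCharacter along the negated normal, overriding XY velocity and adding to Z.
; Disconnected leftovers hold alternative timeline rotation, torque and AddImpulse knockback logic that never runs.
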(event OnComponentHit(KnokbackBall)
  (params (HitComponent :type Primitive%20Component%20Object%20Reference) (OtherActor :type Actor%20Object%20Reference) (OtherComp :type Primitive%20Component%20Object%20Reference) (NormalImpulse :type Vector :default "0, 0, 0") (Hit :type Hit%20Result%20Structure%20%28by%20ref%29))
  (bind _impactnormal (Collision|BreakHitResult Hit))
  (bind (_x _y _z) (Math|Vector|BreakVector _impactnormal))
  (bind _asbp_third_person_character (Utilities|Casting|CastToBP_ThirdPersonCharacter OtherActor))
  (Development|PrintString (Utilities|String|ToString(Vector) _impactnormal))
  (Character|LaunchCharacter _asbp_third_person_character (* (Math|Vector|Normalize (Math|Vector|MakeVector _x _y _z)) -1e+03) true false))

(event EventBeginPlay)

(event Collision|EventActorBeginOverlap
  (params (OtherActor :type Actor%20Object%20Reference))
  (Class|PrimitiveComponent|AddTorqueinDegrees (Variables|Default|GetKnokbackBall) "0.000000,0.000000,10000.000000" "None" false))

(event EventTick
  (params (DeltaSeconds :type Float%20%28single-precision%29)))

(fn ConstructionScript)
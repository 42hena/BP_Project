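; BP_HammerObstacle1 is a rotating hammer obstacle that knocks player characters away.
; Each Tick it spins the actor by RotationSpeed and box-traces from the hammer's previous location to its new one.
; A BP_ThirdPersonCharacter hit is launched horizontally along its world location minus the impact normal, normalized and scaled to a fixed speed.
; The hit normal prints for debugging, and older pivot-rotation logic remains unconnected.
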(event EventBeginPlay)

(event EventTick
  (params (DeltaSeconds :type Float%20%28single-precision%29))
  (bind _hammer (Variables|Default|GetHammer))
  (Variables|Default|SetPreviousLocation (Transformation|GetWorldLocation (Variables|Default|GetHammer)))
  (Class|Actor|AddActorWorldRotation (Math|Rotator|MakeRotator 0.0 0.0 (* DeltaSeconds (Variables|Default|GetRotationSpeed))))
  ;[0.15 0.15 0.15 0.5] Box Trace를 이용하여 충돌처리
  (bind (_outhit _returnvalue) (Collision|BoxTraceByChannel (Variables|Default|GetPreviousLocation) (Transformation|GetWorldLocation _hammer) "25.000000,100.000000,50.000000" (Transformation|GetWorldRotation _hammer) "TraceTypeQuery3" false 0 "ForDuration"))
  (if _returnvalue
    (bind _asbp_third_person_character (Utilities|Casting|CastToBP_ThirdPersonCharacter (.HitActor (Collision|BreakHitResult _outhit))))
    (Development|PrintString (Utilities|String|ToString(Vector) (.Normal (Collision|BreakHitResult _outhit))))
    (Character|LaunchCharacter _asbp_third_person_character (* (Math|Vector|Normalize (Math|Vector|MakeVector (.x (- (Transformation|GetActorLocation (.HitActor (Collision|BreakHitResult _outhit))) (.ImpactNormal (Collision|BreakHitResult _outhit)))) (.y (- (Transformation|GetActorLocation (.HitActor (Collision|BreakHitResult _outhit))) (.ImpactNormal (Collision|BreakHitResult _outhit)))) 0.0)) 1.5e+03) true false)))

(event Collision|EventHit
  (params (MyComp :type Primitive%20Component%20Object%20Reference) (Other :type Actor%20Object%20Reference) (OtherComp :type Primitive%20Component%20Object%20Reference) (bSelfMoved :type Boolean) (HitLocation :type Vector :default "0, 0, 0") (HitNormal :type Vector :default "0, 0, 0") (NormalImpulse :type Vector :default "0, 0, 0") (Hit :type Hit%20Result%20Structure%20%28by%20ref%29)))

(fn ConstructionScript)
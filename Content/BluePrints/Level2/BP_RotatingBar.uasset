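; Rotating bar obstacle for Level 2 that knocks characters away when they touch it.
; Tick spins the Cylinder component around its local yaw at a constant, frame-rate-independent speed.
; Begin-overlap events on three other cylinders feed the sweep's impact normal into a shared PushCharacter event.
; That event casts to Character and applies a mass-independent velocity impulse along the normal.
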(event OnComponentBeginOverlap(Cylinder1)
  (params (OverlappedComponent :type Primitive%20Component%20Object%20Reference) (OtherActor :type Actor%20Object%20Reference) (OtherComp :type Primitive%20Component%20Object%20Reference) (OtherBodyIndex :type Integer) (bFromSweep :type Boolean) (SweepResult :type Hit%20Result%20Structure%20%28by%20ref%29))
  (CallFunction|PushCharacter OtherActor (.ImpactNormal (Collision|BreakHitResult SweepResult))))

(event OnComponentBeginOverlap(Cylinder2)
  (params (OverlappedComponent :type Primitive%20Component%20Object%20Reference) (OtherActor :type Actor%20Object%20Reference) (OtherComp :type Primitive%20Component%20Object%20Reference) (OtherBodyIndex :type Integer) (bFromSweep :type Boolean) (SweepResult :type Hit%20Result%20Structure%20%28by%20ref%29))
  (CallFunction|PushCharacter OtherActor (.ImpactNormal (Collision|BreakHitResult SweepResult))))

(event OnComponentBeginOverlap(Cylinder4)
  (params (OverlappedComponent :type Primitive%20Component%20Object%20Reference) (OtherActor :type Actor%20Object%20Reference) (OtherComp :type Primitive%20Component%20Object%20Reference) (OtherBodyIndex :type Integer) (bFromSweep :type Boolean) (SweepResult :type Hit%20Result%20Structure%20%28by%20ref%29))
  (CallFunction|PushCharacter OtherActor (.ImpactNormal (Collision|BreakHitResult SweepResult))))

(event Custom|PushCharacter
  (params (Other :type Actor%20Object%20Reference) (Normal :type Vector))
  (bind _ascharacter (Utilities|Casting|CastToCharacter Other))
  (Physics|AddImpulse (Variables|/Script/Engine.Character|GetCharacterMovement _ascharacter) (* Normal 1e+02) true))

(event EventBeginPlay)

(event EventTick
  (params (DeltaSeconds :type Float%20%28single-precision%29))
  (Transformation|AddLocalRotation (Variables|Default|GetCylinder) (Math|Rotator|MakeRotator 0.0 0.0 (* DeltaSeconds 6e+01)) false false))

(fn ConstructionScript)
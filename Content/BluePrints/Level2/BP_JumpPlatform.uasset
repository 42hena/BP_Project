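; BP_JumpPlatform is a Level 2 jump platform that launches any Character that hits it upward.
; On Hit it casts the other actor to Character and replaces a downward velocity with a small upward one, discarding horizontal motion.
; It then applies an upward velocity-change impulse through CharacterMovement, ignoring mass.
; Debug prints show the hit actor's name and its vertical velocity.
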(event EventBeginPlay)

(event EventTick
  (params (DeltaSeconds :type Float%20%28single-precision%29)))

(event Collision|EventHit
  (params (MyComp :type Primitive%20Component%20Object%20Reference) (Other :type Actor%20Object%20Reference) (OtherComp :type Primitive%20Component%20Object%20Reference) (bSelfMoved :type Boolean) (HitLocation :type Vector :default "0, 0, 0") (HitNormal :type Vector :default "0, 0, 0") (NormalImpulse :type Vector :default "0, 0, 0") (Hit :type Hit%20Result%20Structure%20%28by%20ref%29))
  (Development|PrintString (Utilities|GetDisplayName Other))
  (bind _ascharacter (Utilities|Casting|CastToCharacter Other))
  (Development|PrintString (Utilities|String|ToString(Float) (.Z (Math|Vector|BreakVector (Variables|/Script/Engine.MovementComponent|GetVelocity (Variables|/Script/Engine.Character|GetCharacterMovement _ascharacter))))))
  (if (< (.Z (Math|Vector|BreakVector (Variables|/Script/Engine.MovementComponent|GetVelocity (Variables|/Script/Engine.Character|GetCharacterMovement _ascharacter)))) 0.0)
    (Variables|/Script/Engine.MovementComponent|SetVelocity (Variables|/Script/Engine.Character|GetCharacterMovement _ascharacter) "0.000000,0.000000,100.000000"))
  (Physics|AddImpulse (Variables|/Script/Engine.Character|GetCharacterMovement _ascharacter) "0.000000,0.000000,600.000000" true))

(fn ConstructionScript)
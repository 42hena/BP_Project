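; BP_MovePlatform2 is a looping moving platform that travels along its own right vector.
; On BeginPlay it caches the Plane's world location, then a Timeline track scaled by a fixed distance offsets the whole actor from that point without sweeping.
; When the Timeline finishes, actor collision turns off for a brief delay, the Timeline restarts from the beginning and collision turns back on.
; Several unconnected leftover chains hold alternative reset and Plane collision logic.
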(event EventBeginPlay
  (Variables|Default|SetInitPos (Transformation|GetWorldLocation (Variables|Default|GetPlane)))
  (bind _testtrack (Timeline|Timeline PlayFromStart)
    (:Update
      (Transformation|SetActorLocation (+ (Variables|Default|GetInitPos) (* (Transformation|GetActorRightVector) _testtrack 1.5e+03)) false false))
    (:Finished
      (Collision|SetActorEnableCollision false)
      (Utilities|FlowControl|Delay 0.05)
      (Components|Timeline|PlayfromStart (Variables|Default|GetTimeline))
      (Collision|SetActorEnableCollision true))))

(event EventTick
  (params (DeltaSeconds :type Float%20%28single-precision%29)))

(fn ConstructionScript)
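; BP_Pusher2 is a moving obstacle that slides between two points and displaces actors it hits.
; After a random startup delay, the PingPong timeline lerps it with sweep from its start location along MoveDirection's forward vector by MoveLength.
; On a blocking hit, it offsets the other actor along the trace line, using the gap between hit distance and full trace length.
; Several older movement, impulse and debug experiments remain unconnected.
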(event EventBeginPlay
  (Utilities|FlowControl|Delay (Math|Random|RandomFloatinRange 0.0 2.0))
  (Variables|Default|SetStartLocation (Transformation|GetActorLocation))
  (Variables|Default|SetEndLocation (+ (Transformation|GetActorLocation) (* (Math|Vector|GetForwardVector (Variables|Default|GetMoveDirection)) (Variables|Default|GetMoveLength))))
  (bind _alpha (Timeline|PingPong Play)
    (:Update
      (Transformation|SetActorLocation (Math|Vector|Lerp(Vector) (Variables|Default|GetStartLocation) (Variables|Default|GetEndLocation) _alpha) true false))))

(event Collision|EventActorBeginOverlap
  (params (OtherActor :type Actor%20Object%20Reference)))

(event Collision|EventHit
  (params (MyComp :type Primitive%20Component%20Object%20Reference) (Other :type Actor%20Object%20Reference) (OtherComp :type Primitive%20Component%20Object%20Reference) (bSelfMoved :type Boolean) (HitLocation :type Vector :default "0, 0, 0") (HitNormal :type Vector :default "0, 0, 0") (NormalImpulse :type Vector :default "0, 0, 0") (Hit :type Hit%20Result%20Structure%20%28by%20ref%29))
  (bind (_bblockinghit _binitialoverlap _time _distance _location _impactpoint _normal _impactnormal _physmat _hitactor _hitcomponent _hitbonename _bonename _hititem _elementindex _faceindex _tracestart _traceend) (Collision|BreakHitResult Hit))
  (if _bblockinghit
    (Transformation|AddActorWorldOffset Other (* (- _distance (Math|Vector|Distance(Vector) _tracestart _traceend)) (Math|Vector|GetUnitDirection(Vector) _tracestart _traceend)) true)))

(event EventTick
  (params (DeltaSeconds :type Float%20%28single-precision%29)))

(fn ConstructionScript)
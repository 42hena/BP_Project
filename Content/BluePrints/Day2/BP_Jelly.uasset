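; BP_Jelly is a slippery surface actor that makes BP_ThirdPersonCharacter and BP_Guy slide while they overlap it.
; On begin overlap it increments the character's Count and lowers CharacterMovement braking, ground friction and acceleration.
; On end overlap it decrements Count and restores hard-coded movement values only when it reaches zero, so overlapping several jellies keeps the slide until the last exit.
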(event EventBeginPlay)

(event Collision|EventActorBeginOverlap
  (params (OtherActor :type Actor%20Object%20Reference))
  (bind _asbp_third_person_character (Utilities|Casting|CastToBP_ThirdPersonCharacter OtherActor)
    (:then
      (Development|PrintString "Start")
      (Variables|/Game/ThirdPerson/Blueprints/BP_ThirdPersonCharacter.BP_ThirdPersonCharacter_C|SetCount _asbp_third_person_character (+ (Variables|/Game/ThirdPerson/Blueprints/BP_ThirdPersonCharacter.BP_ThirdPersonCharacter_C|GetCount _asbp_third_person_character) 1))
      (Variables|/Script/Engine.CharacterMovementComponent|SetBrakingDecelerationWalking (Variables|/Script/Engine.Character|GetCharacterMovement _asbp_third_person_character) 2e+01)
      (Variables|/Script/Engine.CharacterMovementComponent|SetGroundFriction (Variables|/Script/Engine.Character|GetCharacterMovement _asbp_third_person_character) 0.2)
      (Variables|/Script/Engine.CharacterMovementComponent|SetMaxAcceleration (Variables|/Script/Engine.Character|GetCharacterMovement _asbp_third_person_character) 2e+02)
      (Variables|/Script/Engine.CharacterMovementComponent|SetBrakingFrictionFactor (Variables|/Script/Engine.Character|GetCharacterMovement _asbp_third_person_character) 0.0))
    (:CastFailed
      (bind _asbp_guy (Utilities|Casting|CastToBP_Guy OtherActor))
      (Variables|/Game/BluePrints/Character/BP_Guy.BP_Guy_C|SetCount _asbp_guy (+ (Variables|/Game/BluePrints/Character/BP_Guy.BP_Guy_C|GetCount _asbp_guy) 1))
      (Variables|/Script/Engine.CharacterMovementComponent|SetBrakingDecelerationWalking (Variables|/Script/Engine.Character|GetCharacterMovement _asbp_guy) 2e+01)
      (Variables|/Script/Engine.CharacterMovementComponent|SetGroundFriction (Variables|/Script/Engine.Character|GetCharacterMovement _asbp_guy) 0.2)
      (Variables|/Script/Engine.CharacterMovementComponent|SetMaxAcceleration (Variables|/Script/Engine.Character|GetCharacterMovement _asbp_guy) 2e+02)
      (Variables|/Script/Engine.CharacterMovementComponent|SetBrakingFrictionFactor (Variables|/Script/Engine.Character|GetCharacterMovement _asbp_guy) 0.0))))

(event EventTick
  (params (DeltaSeconds :type Float%20%28single-precision%29)))

(event Collision|EventActorEndOverlap
  (params (OtherActor :type Actor%20Object%20Reference))
  (bind _asbp_third_person_character (Utilities|Casting|CastToBP_ThirdPersonCharacter OtherActor)
    (:then
      (Development|PrintString "End")
      (if (== (- (Variables|/Game/ThirdPerson/Blueprints/BP_ThirdPersonCharacter.BP_ThirdPersonCharacter_C|GetCount _asbp_third_person_character) 1) 0)
        (Variables|/Game/ThirdPerson/Blueprints/BP_ThirdPersonCharacter.BP_ThirdPersonCharacter_C|SetCount _asbp_third_person_character (- (Variables|/Game/ThirdPerson/Blueprints/BP_ThirdPersonCharacter.BP_ThirdPersonCharacter_C|GetCount _asbp_third_person_character) 1))
        (Variables|/Script/Engine.CharacterMovementComponent|SetBrakingDecelerationWalking (Variables|/Script/Engine.Character|GetCharacterMovement _asbp_third_person_character) 2048.0)
        (Variables|/Script/Engine.CharacterMovementComponent|SetGroundFriction (Variables|/Script/Engine.Character|GetCharacterMovement _asbp_third_person_character) 8.0)
        (Variables|/Script/Engine.CharacterMovementComponent|SetMaxAcceleration (Variables|/Script/Engine.Character|GetCharacterMovement _asbp_third_person_character) 1.5e+03)
        (Variables|/Script/Engine.CharacterMovementComponent|SetBrakingFrictionFactor (Variables|/Script/Engine.Character|GetCharacterMovement _asbp_third_person_character) 2.0)
        (else
          (Variables|/Game/ThirdPerson/Blueprints/BP_ThirdPersonCharacter.BP_ThirdPersonCharacter_C|SetCount _asbp_third_person_character (- (Variables|/Game/ThirdPerson/Blueprints/BP_ThirdPersonCharacter.BP_ThirdPersonCharacter_C|GetCount _asbp_third_person_character) 1)))))
    (:CastFailed
      (bind _asbp_guy (Utilities|Casting|CastToBP_Guy OtherActor))
      (if (== (- (Variables|/Game/BluePrints/Character/BP_Guy.BP_Guy_C|GetCount _asbp_guy) 1) 0)
        (Variables|/Game/BluePrints/Character/BP_Guy.BP_Guy_C|SetCount _asbp_guy (- (Variables|/Game/BluePrints/Character/BP_Guy.BP_Guy_C|GetCount _asbp_guy) 1))
        (Variables|/Script/Engine.CharacterMovementComponent|SetBrakingDecelerationWalking (Variables|/Script/Engine.Character|GetCharacterMovement _asbp_guy) 2048.0)
        (Variables|/Script/Engine.CharacterMovementComponent|SetGroundFriction (Variables|/Script/Engine.Character|GetCharacterMovement _asbp_guy) 8.0)
        (Variables|/Script/Engine.CharacterMovementComponent|SetMaxAcceleration (Variables|/Script/Engine.Character|GetCharacterMovement _asbp_guy) 1.5e+03)
        (Variables|/Script/Engine.CharacterMovementComponent|SetBrakingFrictionFactor (Variables|/Script/Engine.Character|GetCharacterMovement _asbp_guy) 2.0)
        (else
          (Variables|/Game/BluePrints/Character/BP_Guy.BP_Guy_C|SetCount _asbp_guy (- (Variables|/Game/BluePrints/Character/BP_Guy.BP_Guy_C|GetCount _asbp_guy) 1)))))))

(fn ConstructionScript)
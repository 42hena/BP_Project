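; BP_MoveObstacle is an obstacle actor that moves sideways from its starting position.
; On BeginPlay it stores the Sphere component's world location and starts a timeline.
; Each timeline update sets the actor location to that start point offset along the sphere's right vector, scaled by the timeline track, without sweep.
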(event EventBeginPlay
  (Variables|Default|SetInitPos (Transformation|GetWorldLocation (Variables|Default|GetSphere)))
  (bind _newtrack_0 (Timeline|Timeline PlayFromStart)
    (:Update
      (Transformation|SetActorLocation (+ (Variables|Default|GetInitPos) (* (* (Math|Vector|GetRightVector (Variables|Default|GetSphere)) _newtrack_0) 1e+02)) false false))))

(event Collision|EventActorBeginOverlap
  (params (OtherActor :type Actor%20Object%20Reference)))

(event EventTick
  (params (DeltaSeconds :type Float%20%28single-precision%29)))

(fn ConstructionScript)
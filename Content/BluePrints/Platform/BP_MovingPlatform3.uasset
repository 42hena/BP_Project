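; BP_MovingPlatform3 is a platform actor that acts like a conveyor, pushing the player character along its forward vector without moving itself.
; A box overlap stores and clears the character, and Tick interpolates that character's movement velocity toward a fixed forward speed.
; Debug prints report overlaps and flag very brief ones in red.
; An arrow-directed launch on hit is left disconnected and never runs.
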(event OnComponentBeginOverlap(Box)
  (params (OverlappedComponent :type Primitive%20Component%20Object%20Reference) (OtherActor :type Actor%20Object%20Reference) (OtherComp :type Primitive%20Component%20Object%20Reference) (OtherBodyIndex :type Integer) (bFromSweep :type Boolean) (SweepResult :type Hit%20Result%20Structure%20%28by%20ref%29))
  (bind _asbp_third_person_character (Utilities|Casting|CastToBP_ThirdPersonCharacter OtherActor))
  (Variables|Default|SetActor _asbp_third_person_character)
  (Development|PrintString (Utilities|String|Append "Overlap Begin  Character:" (Utilities|GetDisplayName OtherComp)))
  (Variables|Default|SetOverlapStartTime (Utilities|Time|GetTimeSeconds)))

(event OnComponentEndOverlap(Box)
  (params (OverlappedComponent :type Primitive%20Component%20Object%20Reference) (OtherActor :type Actor%20Object%20Reference) (OtherComp :type Primitive%20Component%20Object%20Reference) (OtherBodyIndex :type Integer))
  (Utilities|Casting|CastToBP_ThirdPersonCharacter OtherActor)
  (Variables|Default|SetActor 0)
  (Development|PrintString (Utilities|String|Append "Overlap End Character:" (Utilities|GetDisplayName OtherComp)))
  (if (<= (- (Utilities|Time|GetTimeSeconds) (Variables|Default|GetOverlapStartTime)) 0.1)
    (Development|PrintString "Hello" true true "(R=1.000000,G=0.000000,B=0.000000,A=1.000000)")))

(event EventBeginPlay
  (Transformation|SetActorLocation (Transformation|GetActorLocation) true false))

(event EventTick
  (params (DeltaSeconds :type Float%20%28single-precision%29))
  (bind _asbp_third_person_character (Utilities|Casting|CastToBP_ThirdPersonCharacter (Variables|Default|GetActor)))
  (Variables|/Script/Engine.MovementComponent|SetVelocity (Variables|/Script/Engine.Character|GetCharacterMovement _asbp_third_person_character) (Math|Interpolation|VInterpTo (Variables|/Script/Engine.MovementComponent|GetVelocity (Variables|/Script/Engine.Character|GetCharacterMovement _asbp_third_person_character)) (* (Transformation|GetActorForwardVector) 2e+02) DeltaSeconds 5.0)))

(event Collision|EventHit
  (params (MyComp :type Primitive%20Component%20Object%20Reference) (Other :type Actor%20Object%20Reference) (OtherComp :type Primitive%20Component%20Object%20Reference) (bSelfMoved :type Boolean) (HitLocation :type Vector :default "0, 0, 0") (HitNormal :type Vector :default "0, 0, 0") (NormalImpulse :type Vector :default "0, 0, 0") (Hit :type Hit%20Result%20Structure%20%28by%20ref%29)))

(event Collision|EventActorBeginOverlap
  (params (OtherActor :type Actor%20Object%20Reference)))

(event Collision|EventActorEndOverlap
  (params (OtherActor :type Actor%20Object%20Reference)))

(fn ConstructionScript)
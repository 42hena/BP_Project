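; BP_Guy is a player character with Enhanced Input movement, look, jump and a mid-air dive.
; A Peace/Jump/Dive state gates actions: jump launches upward from Peace, and dive is available only during Jump.
; Diving launches forward with some carried velocity, tilts the mesh, blocks move input and sets ABP_Guy's Dive flag.
; Landing from Jump or Dive restores the mesh, Peace state and animation flag, with debug prints left in.
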(event Custom|IA_Jump
  ;[0.15 0.15 0.15 0.5] Jump 수정 필요
  (CallFunction|TryJump))

(event Input|EnhancedActionEvents|EnhancedInputActionIA_GuyDive
  (params (ActionValue :type Boolean) (ElapsedSeconds :type Float%20%28double-precision%29) (TriggeredSeconds :type Float%20%28double-precision%29) (InputAction :type Input%20Action%20Object%20Reference :default "/Game/BluePrints/Character/InputAction/IA_GuyDive.IA_GuyDive"))
  (bind _capsulecomponent (Variables|Collision|GetCapsuleComponent))
  (bind _charactermovement (Variables|Character|GetCharacterMovement))
  (bind _returnvalue (Math|Vector|GetForwardVector _capsulecomponent))
  (bind _velocity (Variables|/Script/Engine.MovementComponent|GetVelocity _charactermovement))
  ;[0.15 0.15 0.15 0.5] Comment
  (switch Utilities|FlowControl|Switch|SwitchonEGuyState (Variables|Default|GetBPState)
    (:NewEnumerator1
      (Development|PrintString "Hello"))
    (:NewEnumerator3
      (Variables|Default|SetbBPDive true)
      (Development|PrintString "Dive")
      (Variables|Default|SetBPState "NewEnumerator4")
      (Character|LaunchCharacter (Math|Vector|MakeVector (+ (* (.x _returnvalue) 6e+02) (/ (.x _velocity) 4.0)) (+ (* (.y _returnvalue) 6e+02) (/ (.y _velocity) 4.0)) 1e+02) true false)
      (Transformation|SetRelativeRotation (Variables|Character|GetMesh) "0.000000,-90.000000,70.000000" false false)
      (bind _asabp_guy (Utilities|Casting|CastToABP_Guy (Components|SkeletalMesh|GetAnimInstance (Variables|Character|GetMesh))))
      (Variables|/Game/BluePrints/Character/ABP_Guy.ABP_Guy_C|SetbDive _asabp_guy true))))

(event Input|EnhancedActionEvents|EnhancedInputActionIA_GuyMove
  (params (ActionValue :type Vector%202D%20Structure) (ElapsedSeconds :type Float%20%28double-precision%29) (TriggeredSeconds :type Float%20%28double-precision%29) (InputAction :type Input%20Action%20Object%20Reference :default "/Game/BluePrints/Character/InputAction/IA_GuyMove.IA_GuyMove"))
  ;[0.15 0.15 0.15 0.5] Move Event -> Call Move Function
  (CallFunction|Move ActionValue))

(event Input|EnhancedActionEvents|EnhancedInputActionIA_GuyLook
  (params (ActionValue :type Vector%202D%20Structure) (ElapsedSeconds :type Float%20%28double-precision%29) (TriggeredSeconds :type Float%20%28double-precision%29) (InputAction :type Input%20Action%20Object%20Reference :default "/Game/BluePrints/Character/InputAction/IA_GuyLook.IA_GuyLook"))
  (Pawn|Input|AddControllerYawInput (.x ActionValue)) ; x: left or right then move Yaw
  (Pawn|Input|AddControllerPitchInput (.y ActionValue)) ; y: up or down then move pitch
)

(event Input|EnhancedActionEvents|EnhancedInputActionIA_GuyJump
  (params (ActionValue :type Boolean) (ElapsedSeconds :type Float%20%28double-precision%29) (TriggeredSeconds :type Float%20%28double-precision%29) (InputAction :type Input%20Action%20Object%20Reference :default "/Game/BluePrints/Character/InputAction/IA_GuyJump.IA_GuyJump"))
  ;[0.15 0.15 0.15 0.5] Jump 수정 필요
  (CallFunction|IAJump))

(event EventBeginPlay
  ;[0.15 0.15 0.15 0.5] 향상된 Input system
  (bind _asplayer_controller (Utilities|Casting|CastToPlayerController (Pawn|GetController)))
  (Input|AddMappingContext (PlayerController|LocalPlayerSubsystems|GetEnhancedInputLocalPlayerSubsystem _asplayer_controller) "/Game/BluePrints/Character/IMC_Guy.IMC_Guy" 0 "(bIgnoreAllPressedKeysUntilRelease=True,bForceImmediately=False,bNotifyUserSettings=False)"))

(event EventOnLanded
  (params (Hit :type Hit%20Result%20Structure%20%28by%20ref%29))
  (bind _mesh (Variables|Character|GetMesh))
  (Variables|Default|SetbBPDive false)
  (switch Utilities|FlowControl|Switch|SwitchonEGuyState (Variables|Default|GetBPState)
    (:NewEnumerator3
      _)
    (:NewEnumerator4
      _))
  (Utilities|Casting|CastToABP_Guy (Components|SkeletalMesh|GetAnimInstance _mesh))
  (Transformation|SetRelativeRotation _mesh "0.000000,-90.000000,0.000000" false false)
  (Variables|Default|SetBPState "NewEnumerator1")
  (Development|PrintString "Land!!!")
  (bind _asabp_guy (Utilities|Casting|CastToABP_Guy (Components|SkeletalMesh|GetAnimInstance (Variables|Character|GetMesh))))
  (Variables|/Game/BluePrints/Character/ABP_Guy.ABP_Guy_C|SetbDive _asabp_guy false))

(fn ConstructionScript)

(fn Move
  (params (ActionValue :type Vector%202D%20Structure))
  (bind _returnvalue (Pawn|GetControlRotation :!class /Script/Engine.Pawn))
  (if (not (Variables|Default|GetbBPDive))
    (Pawn|Input|AddMovementInput (+ (* (.x ActionValue) (Math|Vector|GetRightVector (Math|Rotator|MakeRotator (.roll _returnvalue) 0.0 (.yaw _returnvalue)))) (* (.y ActionValue) (Math|Vector|GetForwardVector (Math|Rotator|MakeRotator (.roll _returnvalue) 0.0 (.yaw _returnvalue))))) 1.0 false) ; UE 좌표계로 전환
  ))

(fn LookAround)

(fn TryJump
  (switch Utilities|FlowControl|Switch|SwitchonEGuyState (Variables|Default|GetBPState)
    (:NewEnumerator1
      (Variables|Default|SetBPState "NewEnumerator3")
      (if (not (AI|Components|NavMovement|IsFalling (Variables|Character|GetCharacterMovement)))
        (Character|LaunchCharacter (Math|Vector|MakeVector 0.0 0.0 6e+02) false false)))))